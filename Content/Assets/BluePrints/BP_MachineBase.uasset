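; Base Blueprint for a crystallography machine that analyzes crystal samples once it is calibrated and switched on.
; While off, Tweak slides the gem holder and refraction plate oppositely within limits, checking needle-to-marking alignment for calibration.
; The placeholder overlap snaps crystals in, re-attaching them if pulled out while running.
; OnSwitch drives the laser, status popups and monitor, which receives the crystal's data looked up by name.
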(event OnComponentEndOverlap(SC_PlaceHolder)
  (params (OverlappedComponent :type Primitive%20Component%20Object%20Reference) (OtherActor :type Actor%20Object%20Reference) (OtherComp :type Primitive%20Component%20Object%20Reference) (OtherBodyIndex :type Integer))
  ;[1 1 1] ONOFF
  (if (and (== (Variables|Default|GetisOn) false) (== true (Variables|Default|GetisOccupied)))
    (Utilities|Casting|CastToBP_CrystalBase OtherActor)
    (Variables|Default|SetisOccupied false)
    (Default|ShowMessage (Variables|Default|GetBP_WidgetPopup) "Sample Removed" (Utilities|Struct|MakeSlateColor "(R=1.000000,G=1.000000,B=0.980079,A=1.000000)" "UseColor_Specified"))
    (elif (and (== (Variables|Default|GetisOn) true) (== true (Variables|Default|GetisOccupied)))
      (Default|ShowMessage (Variables|Default|GetBP_WidgetPopup) "!!..Risky...!! 
 
Machine is running,  
Shut it down before removing the sample" (Utilities|Struct|MakeSlateColor "(R=1.000000,G=0.004362,B=0.000000,A=1.000000)" "UseColor_Specified"))
      (Transformation|AttachComponentToComponent (stale OnComponentBeginOverlap(SC_PlaceHolder) _asbp_crystal_base) (Variables|Default|GetSC_PlaceHolder) "None" "SnapToTarget" "SnapToTarget" "SnapToTarget" true)
      (Transformation|SetWorldScale3D (Variables|/Script/Engine.Actor|GetRootComponent (stale OnComponentBeginOverlap(SC_PlaceHolder) _asbp_crystal_base)) (stale OnComponentBeginOverlap(SC_PlaceHolder) _output_get))
      (Variables|Default|SetisOccupied true))))

(event OnComponentBeginOverlap(SC_PlaceHolder)
  (params (OverlappedComponent :type Primitive%20Component%20Object%20Reference) (OtherActor :type Actor%20Object%20Reference) (OtherComp :type Primitive%20Component%20Object%20Reference) (OtherBodyIndex :type Integer) (bFromSweep :type Boolean) (SweepResult :type Hit%20Result%20Structure%20%28by%20ref%29))
  (bind _sc_placeholder (Variables|Default|GetSC_PlaceHolder))
  (bind _sc_placeholder_2 (Variables|Default|GetSC_PlaceHolder))
  ;[1 1 1] ONOFF
  (if (and (== (Variables|Default|GetisOn) false) (== false (Variables|Default|GetisOccupied)))
    ;;[1 0 0 1 15] Disable Crystal Grab Component if machine On and Enable if Off
    (bind _asbp_crystal_base (Utilities|Casting|CastToBP_CrystalBase OtherActor))
    (Variables|Default|SetCrystal _asbp_crystal_base)
    (bind _output_get (Variables|Default|SetCrystalOriginalScale (* (Transformation|GetWorldScale _sc_placeholder) "2.000000,2.000000,2.000000")))
    (Transformation|DetachFromComponent (Variables|/Script/Engine.Actor|GetRootComponent _asbp_crystal_base) "KeepWorld" "KeepWorld" "KeepWorld" true)
    (Transformation|SetWorldLocationAndRotation (Variables|/Game/Assets/BluePrints/Crystals/BP_CrystalBase.BP_CrystalBase_C|GetDefaultSceneRoot _asbp_crystal_base) (Transformation|GetWorldLocation _sc_placeholder_2) (Transformation|GetWorldRotation _sc_placeholder_2) false false)
    ;;[0.49 1 0.9468] AUDIO
    (Audio|PlaySoundatLocation "/Game/Assets/Sound/Stone.Stone" (Transformation|GetWorldLocation (Variables|Default|GetSC_PlaceHolder)) "0, 0, 0" (Variables|Default|GetVolume%20Multiplier) 1.0 0.0 0 0 0 0)
    (Utilities|FlowControl|Delay 1.0)
    (Default|ShowMessage (Variables|Default|GetBP_WidgetPopup) "Sample Detected" (Utilities|Struct|MakeSlateColor "(R=1.000000,G=1.000000,B=1.000000,A=1.000000)" "UseColor_Specified"))
    (Transformation|AttachComponentToComponent _asbp_crystal_base _sc_placeholder "None" "SnapToTarget" "SnapToTarget" "SnapToTarget" true)
    (Transformation|SetWorldScale3D (Variables|/Script/Engine.Actor|GetRootComponent _asbp_crystal_base) _output_get)
    (Variables|Default|SetisOccupied true)))

(event EventBeginPlay
  ;[1 1 1] MonitorONOFF
  (Variables|Default|SetTags (Variables|Default|GetSetMyTag))
  (Default|Switchon (Variables|Default|GetBP_Monitor) (Variables|Default|GetisOn) false)
  (Rendering|SetVisibility (Variables|Default|GetLazer) false false))

(event EventTweak
  (params (Tweak :type Float%20%28double-precision%29))
  (bind _volume_multiplier (Variables|Default|GetVolume%20Multiplier))
  (bind _crystallography_machine_sm_gem_holder (Variables|Default|GetCrystallography_Machine_SM_Gem_Holder))
  (bind _crystallography_machine_sm_gem_holder_2 (Variables|Default|GetCrystallography_Machine_SM_Gem_Holder))
  (bind _crystallography_machine_sm_refraction_plate (Variables|Default|GetCrystallography_Machine_SM_Refraction_Plate))
  (bind _machine_speed (Variables|Default|GetMachine_Speed))
  (bind _returnvalue (Math|Float|Absolute(Float) _machine_speed))
  (bind _relativelocation (Variables|/Script/Engine.SceneComponent|GetRelativeLocation _crystallography_machine_sm_gem_holder_2))
  (bind _returnvalue_2 (* _returnvalue -1.0))
  ;[1 1 1] Mechanics
  ;;[1 1 1] Caliberate
  (if (Variables|Default|GetisOn)
    (Variables|Default|SetisPlaying false)
    (Default|ShowMessage (Variables|Default|GetBP_WidgetPopup) "Can't Calibrate while the Machine is ON" (Utilities|Struct|MakeSlateColor "(R=1.000000,G=1.000000,B=1.000000,A=1.000000)" "UseColor_Specified"))
    (else
      (Variables|Default|SetisPlaying true)
      (if (and (>= (.x _relativelocation) (.x (Variables|/Script/Engine.SceneComponent|GetRelativeLocation (Variables|Default|GetClamp2)))) (<= (.x _relativelocation) (.x (Variables|/Script/Engine.SceneComponent|GetRelativeLocation (Variables|Default|GetClamp1)))))
        (if (> Tweak 0.0)
          (if (> (* (+ _returnvalue 3e+01) -1.0) (.x _relativelocation))
            (Transformation|AddRelativeLocation _crystallography_machine_sm_gem_holder (Math|Vector|MakeVector _returnvalue 0.0 0.0) false false)
            (Transformation|AddRelativeLocation _crystallography_machine_sm_refraction_plate (Math|Vector|MakeVector _returnvalue_2 0.0 0.0) false false)
            ;;[0.49 1 0.9468] AUDIO
            (bind _returnvalue_3 (Audio|SpawnSoundatLocation "/Game/Assets/Sound/Machine.Machine" (Transformation|GetWorldLocation (Variables|Default|GetClamp1)) "0, 0, 0" _volume_multiplier -2.0 0.0 0 0 false :!label _label))
            (Audio|Components|Audio|StopDelayed _returnvalue_3 0.5)
            (else
              (bind _returnvalue_4 (Audio|SpawnSoundatLocation "/Game/Assets/Sound/Machine.Machine" (Transformation|GetWorldLocation (Variables|Default|GetClamp1)) "0, 0, 0" _volume_multiplier 1.0 0.0 0 0 false :!label _label_2))
              (Audio|Components|Audio|StopDelayed _returnvalue_4 0.1)))
          (Variables|Default|SetIsCaliberated (Math|Float|NearlyEqual(Float) (.x (Transformation|GetWorldLocation (Variables|Default|GetCaliberate%20Marking))) (.x (Transformation|GetWorldLocation (Variables|Default|GetCaliberate%20Needle))) 3.0))
          (elif (< Tweak 0.0)
            (if (< (* (- 65.0 _returnvalue) -1.0) (.x _relativelocation))
              (Transformation|AddRelativeLocation _crystallography_machine_sm_gem_holder (Math|Vector|MakeVector _returnvalue_2 0.0 0.0) false false)
              (Transformation|AddRelativeLocation _crystallography_machine_sm_refraction_plate (Math|Vector|MakeVector _returnvalue 0.0 0.0) false false)
              (goto _label)
              (else
                (goto _label_2)))))))))

(event EventSwitchonOff
  (params (IsOn :type Boolean))
  ;[1 1 1] Switch
  (CallFunction|OnSwitch IsOn))

(fn ConstructionScript)

(fn OnSwitch
  (params (isOn :type Boolean))
  (bind _crystaldata (Variables|Default|GetCrystalData))
  (bind _crystal (Variables|Default|GetCrystal))
  (bind _bp_widgetpopup (Variables|Default|GetBP_WidgetPopup))
  (bind _name (Variables|/Game/Assets/BluePrints/Crystals/BP_CrystalBase.BP_CrystalBase_C|GetName _crystal))
  (bind (_value _returnvalue) (Utilities|Map|Find _crystaldata _name))
  (bind _output_get (Variables|Default|SetisOn isOn))
  (if _output_get
    (if (Variables|Default|GetisOccupied)
      (if _returnvalue
        (if (Variables|Default|GetIsCaliberated)
          (Default|Switchon (Variables|Default|GetBP_Monitor) true (Variables|Default|GetisOccupied))
          (Default|OnDataUpdate (Variables|Default|GetBP_Monitor) _value)
          (Default|HideMessage (Variables|Default|GetBP_WidgetPopup))
          (Rendering|SetVisibility (Variables|Default|GetLazer) true false)
          (else
            (Default|ShowMessage (Variables|Default|GetBP_WidgetPopup) "Calibration Needed" (Utilities|Struct|MakeSlateColor "(R=1.000000,G=1.000000,B=1.000000,A=1.000000)" "UseColor_Specified")))))
      (else
        (Default|Switchon (Variables|Default|GetBP_Monitor) true false)
        (if (Variables|Default|GetIsCaliberated)
          (Default|ShowMessage _bp_widgetpopup "Calibrated but No Sample Detected" (Utilities|Struct|MakeSlateColor "(R=1.000000,G=1.000000,B=1.000000,A=1.000000)" "UseColor_Specified"))
          (else
            (Default|ShowMessage _bp_widgetpopup "Calibration and Sample Needed" (Utilities|Struct|MakeSlateColor "(R=1.000000,G=1.000000,B=1.000000,A=1.000000)" "UseColor_Specified"))))))
    (else
      (Default|HideMessage (Variables|Default|GetBP_WidgetPopup))
      (Default|Switchon (Variables|Default|GetBP_Monitor) false false)
      (Rendering|SetVisibility (Variables|Default|GetLazer) false false)
      (if (not (or (Variables|Default|GetIsCaliberated) (Variables|Default|GetisOccupied)))
        (Default|ShowMessage (Variables|Default|GetBP_WidgetPopup) " Follow the Steps" (Utilities|Struct|MakeSlateColor "(R=1.000000,G=1.000000,B=1.000000,A=1.000000)" "UseColor_Specified"))))))