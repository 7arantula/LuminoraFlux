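; BP_LeftHand is a left-hand motion controller Blueprint that passes its components to another actor for grab handling.
; On BeginPlay it sets its tags, waits briefly, then searches actors implementing BPI_GrabResponse and caches one tagged "Hand", keeping the last match.
; Its SendResponse event calls SendForGrabMessage on that cached actor, handing over the motion controller, controller mesh and knob follow target.
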(event EventBeginPlay
  (Variables|Default|SetTags (Variables|Default|GetTags_0))
  (Utilities|FlowControl|Delay 0.2)
  (bind _outactors (Actor|GetAllActorswithInterface "/Game/Assets/BluePrints/BPI_GrabResponse.BPI_GrabResponse_C"))
  (for _array_element _outactors
    (if (Actor|ActorHasTag _array_element "Hand")
      (Variables|Default|SetArray%20Element _array_element))))

(event EventSendResponse
  (Class|BPICaliberate|SendforGrab(Message) (Variables|Default|GetArray%20Element) (Variables|Default|GetMotionController) (Variables|Default|GetControllerMesh) (Variables|Default|GetKnobFollowTarget)))

(fn ConstructionScript)