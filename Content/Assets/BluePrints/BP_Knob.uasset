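; BP_Knob is a hand-turned calibration knob that tweaks a machine and gives detent-style haptic ticks.
; After a short delay, BeginPlay finds the BPI_Caliberate actor tagged "Machine" and opens a gate driven by Tick.
; Gated yaw comparisons send +1 or -1 TweakMessage calls as the knob turns.
; Tick arms haptics near ten-degree steps, picking the hand from the owner of the component attached to Arrow.
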(event EventBeginPlay
  ;[0.4996 1 0.4991] Find Machine
  (Variables|Default|SetTags (Variables|Default|GetSetMyTags))
  (Utilities|FlowControl|Delay 0.2)
  (bind _outactors (Actor|GetAllActorswithInterface "/Game/Assets/BluePrints/BPI_Caliberate.BPI_Caliberate_C"))
  (for _array_element _outactors
    (if (Actor|ActorHasTag _array_element "Machine")
      (Variables|Default|SetElementMachine _array_element)
      ;[0.4288 0.475 1] SetChange
      (Utilities|FlowControl|Gate true) ; enters at Open
    )))

(event EventTick
  (params (DeltaSeconds :type Float%20%28single-precision%29))
  (bind _knob_sm_knob (Variables|Default|GetKnob_SM_Knob))
  (bind _arrow (Variables|Default|GetArrow))
  (bind _elementmachine (Variables|Default|GetElementMachine))
  (bind _returnvalue (Components|GetChildComponent _arrow 0))
  (bind _relativerotation (Variables|/Script/Engine.SceneComponent|GetRelativeRotation _knob_sm_knob))
  (bind _returnvalue_2 (Components|GetOwner _returnvalue))
  (bind _returnvalue_3 (/ (.yaw _relativerotation) 1e+01))
  ;[0.4288 0.475 1] SetChange
  (if (and (Math|Float|NearlyEqual(Float) _returnvalue_3 (Math|Conversions|ToFloat(Integer) (Class|KismetMathLibrary|FTrunc64 _returnvalue_3)) 0.1) (Utilities|IsValid _returnvalue))
    (Variables|Default|SetPlayHaptic true)
    (Utilities|Casting|CastToBP_LeftHand _returnvalue_2
      (:then
        (Variables|Default|SetHand "Left"))
      (:CastFailed
        (Utilities|Casting|CastToBP_RightHand _returnvalue_2
          (:then
            (Variables|Default|SetHand "Right"))
          (:CastFailed
            (Variables|Default|SetHand "HMD")))))
    (else
      (Utilities|FlowControl|Gate true
        (:Exit
          (bind _output_get (Variables|Default|SetCurrentRotation (Transformation|GetWorldRotation (Variables|Default|GetKnob_SM_Knob))))
          (if (> (.yaw _output_get) (.yaw (Variables|Default|GetPreviousRotation)))
            (Class|BPICaliberate|Tweak(Message) _elementmachine 1.0)
            (Variables|Default|SetPreviousRotation (Variables|Default|GetCurrentRotation))
            (if (Variables|Default|GetPlayHaptic) :!label _label
              (Class|PlayerController|PlayHapticEffect (Game|GetPlayerController 0) "/Game/Assets/Haptics/Tick.Tick" (Variables|Default|GetHand) 5.0 false)
              (Variables|Default|SetPlayHaptic false))
            (elif (not (== (.yaw _output_get) (.yaw (Variables|Default|GetPreviousRotation))))
              (Class|BPICaliberate|Tweak(Message) _elementmachine -1.0)
              (Variables|Default|SetPreviousRotation (Variables|Default|GetCurrentRotation))
              (goto _label))))))))

(fn ConstructionScript)