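; BP_Tray is a tray actor that snaps crystals placed on it into fixed slots.
; When a crystal actor overlaps its Box, it reads the crystal's Name and picks a position offset from the Tray component for Diamond, Quartz or NaCl.
; It then attaches the crystal to the Tray with snap rules and moves it to that position.
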(event OnComponentBeginOverlap(Box)
  (params (OverlappedComponent :type Primitive%20Component%20Object%20Reference) (OtherActor :type Actor%20Object%20Reference) (OtherComp :type Primitive%20Component%20Object%20Reference) (OtherBodyIndex :type Integer) (bFromSweep :type Boolean) (SweepResult :type Hit%20Result%20Structure%20%28by%20ref%29))
  (bind _tray (Variables|Default|GetTray))
  (bind _returnvalue (Transformation|GetWorldLocation _tray))
  (bind _asbp_crystal_base (Utilities|Casting|CastToBP_CrystalBase OtherActor))
  (bind _output_get (Variables|Default|SetAs%20BP%20Crystal%20Base _asbp_crystal_base))
  (Variables|Default|SetCrystal (Variables|/Game/Assets/BluePrints/Crystals/BP_CrystalBase.BP_CrystalBase_C|GetName (Variables|Default|GetAs%20BP%20Crystal%20Base)))
  (switch Utilities|FlowControl|Switch|SwitchonECrystals (Variables|Default|GetCrystal)
    (:NewEnumerator0
      (Variables|Default|SetPlacement (+ _returnvalue "0.000000,0.000000,0.000000")))
    (:NewEnumerator1
      (Variables|Default|SetPlacement (+ _returnvalue "25.000000,0.000000,0.000000")))
    (:NewEnumerator2
      (Variables|Default|SetPlacement (+ _returnvalue "-25.000000,0.000000,1.000000"))))
  (Transformation|AttachComponentToComponent _output_get _tray "None" "SnapToTarget" "SnapToTarget" "SnapToTarget" true)
  (Transformation|SetWorldLocation (Variables|/Script/Engine.Actor|GetRootComponent (Variables|Default|GetAs%20BP%20Crystal%20Base)) (Variables|Default|GetPlacement) false false))

(fn ConstructionScript)