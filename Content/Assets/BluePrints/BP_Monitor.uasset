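; BP_Monitor is a two-screen monitor that displays crystal data: a graph, a pattern and the crystal's name.
; SwitchOn creates dynamic screen materials from MT_ScreenMaster when on and occupied, or restores static materials when off, as at BeginPlay.
; OnDataUpdate feeds the graph and pattern textures into those materials and shows the name in a popup widget, which SwitchOn hides.
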(event EventBeginPlay
  (CallFunction|Switchon false false))

(fn ConstructionScript)

(fn OnDataUpdate
  (params (Crystal%20Data :type Struct%20Crystal%20Data%20Structure))
  (bind (_ename _name _graph _pattern) (Utilities|Struct|BreakStruct_CrystalData Crystal%20Data))
  (Rendering|Material|SetTextureParameterValue (Variables|Default|GetMT_Screen1) "Image Texture" _graph)
  (Rendering|Material|SetTextureParameterValue (Variables|Default|GetMT_Screen2) "Image Texture" _pattern)
  (Default|ShowMessage (Variables|Default|GetBP_WidgetPopup) _name (Variables|Default|GetColor)))

(fn Switchon
  (params (isOn :type Boolean) (isOccupied :type Boolean))
  (Default|HideMessage (Variables|Default|GetBP_WidgetPopup))
  (bind _output_get (Variables|Default|SetisOn isOn))
  (if _output_get
    (if isOccupied
      (bind _returnvalue (Rendering|Material|CreateDynamicMaterialInstance (Variables|Default|GetMonitor_Decals_SM_Screen1) 0 "/Game/Assets/Materials/MT_ScreenMaster.MT_ScreenMaster" "None" :!class /Script/Engine.PrimitiveComponent))
      (Variables|Default|SetMT_Screen1 _returnvalue)
      (bind _returnvalue_2 (Rendering|Material|CreateDynamicMaterialInstance (Variables|Default|GetMonitor_Decals_SM_Screen2) 0 "/Game/Assets/Materials/MT_ScreenMaster.MT_ScreenMaster" "None" :!class /Script/Engine.PrimitiveComponent))
      (Variables|Default|SetMT_Screen2 _returnvalue_2))
    (else
      (Rendering|Material|SetMaterial (Variables|Default|GetMonitor_Decals_SM_Screen1) 0 "/Game/Assets/Meshes/Machines/T_X-Ray_Monitor/M_Screen1.M_Screen1")
      (Rendering|Material|SetMaterial (Variables|Default|GetMonitor_Decals_SM_Screen2) 0 "/Game/Assets/Meshes/Machines/T_X-Ray_Monitor/M_Screen2.M_Screen2")
      (Default|HideMessage (Variables|Default|GetBP_WidgetPopup)))))