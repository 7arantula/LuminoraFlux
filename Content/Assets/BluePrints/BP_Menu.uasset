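; BP_Menu is an actor that shows a menu widget reflecting the state of a machine in the level.
; On BeginPlay it scans all actors for the "Machine" tag and casts each match to BP_MachineBase.
; The machine's calibrated, occupied and on flags set the visibility of three check marks in WB_Menu.
; It then plays the Grow timeline, which scales the Flash component.
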(event EventBeginPlay
  (bind _aswb_menu (Utilities|Casting|CastToWB_Menu (UserInterface|GetWidget (Variables|Default|GetMenuWidget))))
  (Variables|Default|SetAs%20WB%20Menu _aswb_menu)
  (bind _outactors (Actor|GetAllActorsOfClass "/Script/Engine.Actor"))
  (for _array_element _outactors
    (if (Actor|ActorHasTag _array_element "Machine")
      (bind _output_get (Variables|Default|SetMachine _array_element))
      (bind _asbp_machine_base (Utilities|Casting|CastToBP_MachineBase _output_get))
      (Variables|Default|SetAs%20BP%20Machine%20Base _asbp_machine_base)
      (if (Variables|/Game/Assets/BluePrints/BP_MachineBase.BP_MachineBase_C|GetIsCaliberated (Variables|Default|GetAs%20BP%20Machine%20Base))
        (Widget|SetVisibility (Variables|/Game/Assets/UI/WB_Menu.WB_Menu_C|GetC-Check (Variables|Default|GetAs%20WB%20Menu)) "Visible")
        (else
          (Widget|SetVisibility (Variables|/Game/Assets/UI/WB_Menu.WB_Menu_C|GetC-Check (Variables|Default|GetAs%20WB%20Menu)) "Hidden")))
      (if (Variables|/Game/Assets/BluePrints/BP_MachineBase.BP_MachineBase_C|GetisOccupied (Variables|Default|GetAs%20BP%20Machine%20Base))
        (Widget|SetVisibility (Variables|/Game/Assets/UI/WB_Menu.WB_Menu_C|GetG-Check (Variables|Default|GetAs%20WB%20Menu)) "Visible")
        (else
          (Widget|SetVisibility (Variables|/Game/Assets/UI/WB_Menu.WB_Menu_C|GetG-Check (Variables|Default|GetAs%20WB%20Menu)) "Hidden")))
      (if (Variables|/Game/Assets/BluePrints/BP_MachineBase.BP_MachineBase_C|GetisOn (Variables|Default|GetAs%20BP%20Machine%20Base))
        (Widget|SetVisibility (Variables|/Game/Assets/UI/WB_Menu.WB_Menu_C|GetM-Check (Variables|Default|GetAs%20WB%20Menu)) "Visible")
        (bind (_direction _size _height) (Timeline|Grow Play)
          (:Update
            (Transformation|SetRelativeScale3D (Variables|Default|GetFlash) (Math|Vector|MakeVector _size _size _height))))
        (else
          (Widget|SetVisibility (Variables|/Game/Assets/UI/WB_Menu.WB_Menu_C|GetM-Check (Variables|Default|GetAs%20WB%20Menu)) "Hidden")
          (Timeline|Grow Play))))))

(fn ConstructionScript)