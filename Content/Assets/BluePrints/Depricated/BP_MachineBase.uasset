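; Machine base Blueprint, filed as deprecated, for a crystallography machine with movable gem holder, refraction plate and nozzle meshes.
; BeginPlay sets its tags, and a Tweak event slides the three parts along X by remapping the input from a symmetric range, with the plate's input range reversed relative to the others.
; Clamp components supply the travel limits and fixed Y/Z, except one plate X limit, which uses the raw range value.
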(event EventBeginPlay
  (Variables|Default|SetTags (Variables|Default|GetTags_0)))

(event Collision|EventActorBeginOverlap
  (params (OtherActor :type Actor%20Object%20Reference)))

(event EventTweak
  (params (Tweak :type Float%20%28double-precision%29))
  (bind _clamp2 (Variables|Default|GetClamp2))
  (bind _clamp4 (Variables|Default|GetClamp4))
  (bind _clamp6 (Variables|Default|GetClamp6))
  (bind _negativerangevalue (Variables|Default|GetNegativeRangeValue))
  (bind _returnvalue (Math|Float|Absolute(Float) _negativerangevalue))
  (bind _relativelocation (Variables|/Script/Engine.SceneComponent|GetRelativeLocation _clamp4))
  (bind _relativelocation_2 (Variables|/Script/Engine.SceneComponent|GetRelativeLocation _clamp6))
  (bind _relativelocation_3 (Variables|/Script/Engine.SceneComponent|GetRelativeLocation _clamp2))
  (Transformation|SetRelativeLocation (Variables|Default|GetCrystallography_Machine_SM_Gem_Holder) (Math|Vector|MakeVector (Math|Float|MapRangeClamped Tweak _returnvalue _negativerangevalue (.x _relativelocation_3) (.x (Variables|/Script/Engine.SceneComponent|GetRelativeLocation (Variables|Default|GetClamp1)))) (.y _relativelocation_3) (.z _relativelocation_3)) false false)
  (Transformation|SetRelativeLocation (Variables|Default|GetCrystallography_Machine_SM_Refraction_Plate) (Math|Vector|MakeVector (Math|Float|MapRangeClamped Tweak _negativerangevalue _returnvalue _negativerangevalue (.x (Variables|/Script/Engine.SceneComponent|GetRelativeLocation (Variables|Default|GetClamp3)))) (.y _relativelocation) (.z _relativelocation)) false false)
  (Transformation|SetRelativeLocation (Variables|Default|GetCrystallography_Machine_SM_Nozel) (Math|Vector|MakeVector (Math|Float|MapRangeClamped Tweak _returnvalue _negativerangevalue (.x _relativelocation_2) (.x (Variables|/Script/Engine.SceneComponent|GetRelativeLocation (Variables|Default|GetClamp5)))) (.y _relativelocation_2) (.z _relativelocation_2)) false false))

(fn ConstructionScript)