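; BP_W_Popup is a popup actor that shows a colored text message on a widget component in the world.
; ShowMessage makes the widget visible and passes text and color to its W_PopUp instance, while HideMessage hides it.
; Construction applies the draw size, and BeginPlay applies the visibility flag and plays the FloatInTheAir timeline.
; That timeline offsets the widget's Z from its current value on each update, so movement accumulates.
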(event EventBeginPlay
  (bind _widget (Variables|Default|GetWidget))
  (bind _relativelocation (Variables|/Script/Engine.SceneComponent|GetRelativeLocation _widget))
  (Rendering|SetVisibility (Variables|Default|GetWidget) (Variables|Default|GetVisibility) false)
  (bind _alpha (Timeline|Float%20in%20the%20air Play)
    (:Update
      (Transformation|SetRelativeLocation (Variables|Default|GetWidget) (Math|Vector|MakeVector (.x _relativelocation) (.y _relativelocation) (Math|Float|Lerp (.z _relativelocation) (+ (.z _relativelocation) 0.5) _alpha)) false false))))

(event EventTick
  (params (DeltaSeconds :type Float%20%28single-precision%29)))

(fn ConstructionScript
  (Class|WidgetComponent|SetDrawSize (Variables|Default|GetWidget) (Variables|Default|GetDrawSize)))

(fn ShowMessage
  (params (Text :type Text) (Color :type Slate%20Color%20Structure))
  (bind _widget (Variables|Default|GetWidget))
  (bind _output_get (Variables|Default|SetVisibility true))
  (Rendering|SetVisibility _widget _output_get false)
  (bind _asw_pop_up (Utilities|Casting|CastToW_PopUp (UserInterface|GetWidget _widget)))
  (Variables|/Game/Assets/UI/W_PopUp.W_PopUp_C|SetText _asw_pop_up Text)
  (Variables|/Game/Assets/UI/W_PopUp.W_PopUp_C|SetColor _asw_pop_up Color))

(fn HideMessage
  (bind _output_get (Variables|Default|SetVisibility false))
  (Rendering|SetVisibility (Variables|Default|GetWidget) _output_get false))