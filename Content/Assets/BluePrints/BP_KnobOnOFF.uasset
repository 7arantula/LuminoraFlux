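; VR rotary on/off knob that switches actors tagged Bulb and Machine, found through BPI_Caliberate shortly after BeginPlay.
; Tick feeds a gate that compares knob yaw to the previous value, nudging a clamped threshold to send on or off messages once rotation passes either limit.
; When a child is attached to Arrow near whole-degree yaw, Tick identifies the hand and arms a tick haptic, otherwise switching plays a spring haptic.
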(event EventBeginPlay
  (bind _returnvalue (Game|GetPlayerController 0))
  (bind _hand (Variables|Default|GetHand))
  ;[0.4996 1 0.4991] Find Machine
  (Variables|Default|SetTags (Variables|Default|GetSetMyTags))
  (Utilities|FlowControl|Delay 0.2)
  (bind _outactors (Actor|GetAllActorswithInterface "/Game/Assets/BluePrints/BPI_Caliberate.BPI_Caliberate_C"))
  (for _array_element _outactors
    (if (Actor|ActorHasTag _array_element "Bulb")
      (Variables|Default|SetBulb _array_element)
      ;[0.4288 0.475 1] SetChange
      (Utilities|FlowControl|Gate true) ; enters at Open
      (elif (Actor|ActorHasTag _array_element "Machine")
        (Variables|Default|SetArray%20Element _array_element)
        (Utilities|FlowControl|Gate true) ; enters at Open
      ))))

(event EventTick
  (params (DeltaSeconds :type Float%20%28single-precision%29))
  (bind _returnvalue (Game|GetPlayerController 0))
  (bind _knob_sm_knob (Variables|Default|GetKnob_SM_Knob))
  (bind _arrow (Variables|Default|GetArrow))
  (bind _returnvalue_2 (Components|GetChildComponent _arrow 0))
  (bind _relativerotation (Variables|/Script/Engine.SceneComponent|GetRelativeRotation _knob_sm_knob))
  (bind _returnvalue_3 (Components|GetOwner _returnvalue_2))
  (if (and (Math|Float|NearlyEqual(Float) (.yaw _relativerotation) (Math|Conversions|ToFloat(Integer) (Class|KismetMathLibrary|FTrunc64 (.yaw _relativerotation))) 0.1) (Utilities|IsValid _returnvalue_2))
    (Variables|Default|SetPlayHaptic true)
    (Utilities|Casting|CastToBP_LeftHand _returnvalue_3
      (:then
        (Variables|Default|SetHand "Left"))
      (:CastFailed
        (Utilities|Casting|CastToBP_RightHand _returnvalue_3
          (:then
            (Variables|Default|SetHand "Right"))
          (:CastFailed
            (Variables|Default|SetHand "HMD")))))
    (else
      ;[0.4288 0.475 1] SetChange
      (Utilities|FlowControl|Gate true
        (:Exit
          (bind _output_get (Variables|Default|SetCurrentRotation (Transformation|GetWorldRotation (Variables|Default|GetKnob_SM_Knob))))
          (if (> (.yaw _output_get) (.yaw (Variables|Default|GetPreviousRotation)))
            (Variables|Default|SetThresh (+ 0.5 (Variables|Default|GetThresh)))
            (if (> (Variables|Default|GetThresh) 5.0)
              (Class|BPICaliberate|SwitchonOff(Message) (Variables|Default|GetBulb) true)
              (Class|BPICaliberate|SwitchonOff(Message) (Variables|Default|GetArray%20Element) true)
              (Variables|Default|SetPreviousRotation (Variables|Default|GetCurrentRotation))
              (if (> (Variables|Default|GetThresh) 1e+01)
                (Variables|Default|SetThresh 1e+01))
              (if (Variables|Default|GetPlayHaptic) :!label _label
                (Class|PlayerController|PlayHapticEffect _returnvalue "/Game/Assets/Haptics/Tick.Tick" (Variables|Default|GetHand) 5.0 false)
                (Variables|Default|SetPlayHaptic false)
                (else
                  (Class|PlayerController|PlayHapticEffect _returnvalue "/Game/Assets/Haptics/Spring.Spring" (Variables|Default|GetHand) 3.0 false))))
            (elif (not (== (.yaw _output_get) (.yaw (Variables|Default|GetPreviousRotation))))
              (Variables|Default|SetThresh (+ -0.5 (Variables|Default|GetThresh)))
              (if (< (Variables|Default|GetThresh) -5.0)
                (Class|BPICaliberate|SwitchonOff(Message) (Variables|Default|GetBulb) false)
                (Class|BPICaliberate|SwitchonOff(Message) (Variables|Default|GetArray%20Element) false)
                (Variables|Default|SetPreviousRotation (Variables|Default|GetCurrentRotation))
                (if (< (Variables|Default|GetThresh) -1e+01)
                  (Variables|Default|SetThresh -1e+01)
                  (goto _label)
                  (else
                    (goto _label)))))))))))

(fn ConstructionScript)